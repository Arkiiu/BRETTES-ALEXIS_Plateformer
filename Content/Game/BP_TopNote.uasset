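; BP_TopNote is a note actor, apparently for a rhythm game, that travels along negative X at a height shared through the game instance.
; BeginPlay caches BP_RythmInstance, and Tick teleports the Cube and root, keeping Y from the Cube and taking Z from the instance's TopNoteHeight.
; X movement uses FInterpTo toward one unit behind the current position each frame, scaled by NoteSpeed.
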(event `self.ReceiveBeginPlay`
  (bind _asbp_rythm_instance (cast `/Game/Game/GameInstances/BP_RythmInstance` (`GameplayStatics.GetGameInstance`)))
  (bind _output_get (set `self.BP Rythm Instance` _asbp_rythm_instance)))

(event `self.ReceiveTick`
  (params (DeltaSeconds :type "Float (single-precision)"))
  (bind _cube (`self.Cube`))
  (bind (_returnvalue_x _returnvalue_y) (`KismetMathLibrary.BreakVector` (`SceneComponent.K2_GetComponentLocation` _cube)))
  (`SceneComponent.K2_SetWorldLocation` _cube (`KismetMathLibrary.MakeVector` (`KismetMathLibrary.FInterpTo` _returnvalue_x (- _returnvalue_x 1.0) DeltaSeconds (`self.NoteSpeed`)) _returnvalue_y (`/Game/Game/GameInstances/BP_RythmInstance.TopNoteHeight` (`self.BP Rythm Instance`))) false true)
  (`SceneComponent.K2_SetWorldLocation` (`self.DefaultSceneRoot`) (`KismetMathLibrary.MakeVector` (`KismetMathLibrary.FInterpTo` _returnvalue_x (- _returnvalue_x 1.0) DeltaSeconds (`self.NoteSpeed`)) _returnvalue_y (`/Game/Game/GameInstances/BP_RythmInstance.TopNoteHeight` (`self.BP Rythm Instance`))) false true))

(fn `UserConstructionScript`)