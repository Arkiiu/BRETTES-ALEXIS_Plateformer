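; Player component that tracks bonus charge from collectibles and spends it on a score multiplier, with state held in BP_GameInstance.
; CollectBonusCharge adds a collectible's value to the stored charge and destroys it, but on overflow caps the charge at five and leaves the collectible in place.
; The IA_ScoreMultiplier input calls the game instance's ScoreMultiply only when the charge is exactly full.
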(event `self.ReceiveBeginPlay`
  (bind _asbp_game_instance (cast `/Game/Blueprint/BP_GameInstance` (`GameplayStatics.GetGameInstance`)))
  (set `self.BP Game Instance` _asbp_game_instance))

(event `self.ReceiveTick`
  (params (DeltaSeconds :type "Float (single-precision)")))

(event `EnhancedInput|/Game/ThirdPerson/Input/Actions/IA_ScoreMultiplier`
  (params (ActionValue :type Boolean) (ElapsedSeconds :type "Float (double-precision)") (TriggeredSeconds :type "Float (double-precision)") (InputAction :type "InputAction Object Reference" :default "/Game/ThirdPerson/Input/Actions/IA_ScoreMultiplier.IA_ScoreMultiplier"))
  (bind _bp_game_instance (`self.BP Game Instance`))
  (:`Triggered`
    (if (== (`/Game/Blueprint/BP_GameInstance.BonusCharge` _bp_game_instance) 5)
      (`/Game/Blueprint/BP_GameInstance.ScoreMultiply` _bp_game_instance))))

(fn `CollectBonusCharge`
  (params (Collectible :type "/Game/Blueprint/BPC_CollectibleBonusComponent Object Reference"))
  (bind _bp_game_instance (`self.BP Game Instance`))
  (bind _output_get (set `/Game/Blueprint/BP_GameInstance.BonusCharge` (+ (`/Game/Blueprint/BPC_CollectibleBonusComponent.BonusValue` Collectible) (`/Game/Blueprint/BP_GameInstance.BonusCharge` _bp_game_instance)) _bp_game_instance))
  (if (not (>= _output_get 6))
    (`/Game/Blueprint/BPC_CollectibleBonusComponent.DestroyBPCollectible` Collectible)
    (else
      (set `/Game/Blueprint/BP_GameInstance.BonusCharge` 5 _bp_game_instance))))