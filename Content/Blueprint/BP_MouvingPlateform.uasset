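; A moving platform Blueprint that shifts its Cube component along a straight diagonal path when play begins.
; BeginPlay stores the cube's world location, then plays the Movement timeline.
; Each timeline update linearly interpolates the cube toward a fixed offset along negative X and upward in Z, keeping Y constant.
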(event `self.ReceiveBeginPlay`
  (bind _cube (`self.Cube`))
  (bind _x (.x (`self.Loc`)))
  (bind _z (.z (`self.Loc`)))
  (set `self.Loc` (`SceneComponent.K2_GetComponentLocation` _cube))
  (bind (_direction _newtrack_0) (`Timeline|Movement`)
    (:`Update`
      (`SceneComponent.K2_SetWorldLocation` _cube (`KismetMathLibrary.MakeVector` (`|EaseFunction` "Linear" _newtrack_0 _x (- _x 400.0)) (.y (`self.Loc`)) (`|EaseFunction` "Linear" _newtrack_0 _z (+ _z 150.0))) false false))))

(fn `UserConstructionScript`)