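; BP_Player is the player Blueprint, which creates the main HUD, caches the game instance and handles overlaps with collectibles and interactables.
; Each overlap sets the game instance's CanPress and CanPressLight flags by checking for interactable components, clearing them only when a later overlap lacks one.
; It then passes any collectible component to the collect component, or otherwise any bonus collectible to the bonus collect component.
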(event `self.ReceiveBeginPlay`
  (`parent.ReceiveBeginPlay`)
  (bind _returnvalue (`|CreateWidget` "/Game/Blueprint/WBP_MainHUD.WBP_MainHUD_C"))
  (`UserWidget.AddToViewport` _returnvalue 0)
  (bind _asbp_game_instance (cast `/Game/Game/GameInstances/BP_GameInstance` (`GameplayStatics.GetGameInstance`)))
  (set `self.BP Game Instance` _asbp_game_instance))

(event `self.ReceiveActorBeginOverlap`
  (params (OtherActor :type "Actor Object Reference"))
  (`self. Interact` OtherActor)
  (`self.CollectObject` OtherActor))

(fn ` Interact`
  (params (Actor :type "Actor Object Reference"))
  (bind _bp_game_instance (`self.BP Game Instance`))
  (`|ExecutionSequence`
    (:`then_0`
      (`/Engine/EditorBlueprintResources/StandardMacros.IsValid` (`self.GetComponentByClass` Actor "/Game/Blueprint/BPC_Interactable.BPC_Interactable_C")
        (:`Is Valid`
          (set `/Game/Game/GameInstances/BP_GameInstance.CanPress? ` true _bp_game_instance))
        (:`Is Not Valid`
          (set `/Game/Game/GameInstances/BP_GameInstance.CanPress? ` false _bp_game_instance))))
    (:`then_1`
      (`/Engine/EditorBlueprintResources/StandardMacros.IsValid` (`self.GetComponentByClass` Actor "/Game/Blueprint/BPC_InteractableLight.BPC_InteractableLight_C")
        (:`Is Valid`
          (set `/Game/Game/GameInstances/BP_GameInstance.CanPressLight?` true _bp_game_instance))
        (:`Is Not Valid`
          (set `/Game/Game/GameInstances/BP_GameInstance.CanPressLight?` false _bp_game_instance))))))

(fn `CollectObject`
  (params (OtherActor :type "Actor Object Reference"))
  (bind _returnvalue (`self.GetComponentByClass` OtherActor "/Game/Blueprint/BPC_CollectibleComponent.BPC_CollectibleComponent_C"))
  (bind _returnvalue_2 (`self.GetComponentByClass` OtherActor "/Game/Blueprint/BPC_CollectibleBonusComponent.BPC_CollectibleBonusComponent_C"))
  (`/Engine/EditorBlueprintResources/StandardMacros.IsValid` _returnvalue
    (:`Is Valid`
      (`/Game/Blueprint/BPC_CollectComponent.Collect` (`self.BPC_CollectComponent`) _returnvalue))
    (:`Is Not Valid`
      (`/Engine/EditorBlueprintResources/StandardMacros.IsValid` _returnvalue_2
        (:`Is Valid`
          (`/Game/Blueprint/BPC_CollectBonusComponent.CollectBonusCharge` (`self.BPC_CollectBonusComponent`) _returnvalue_2))))))

(fn `UserConstructionScript`
  (`parent.UserConstructionScript`))