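; BPC_Interacter is an interaction component that turns the interact input into button presses on the game instance.
; It caches BP_GameInstance on BeginPlay.
; When IA_Interact starts, it calls ButtonPressed if CanPress is set, otherwise ButtonPressedLight if CanPressLight is set.
; All press state and resulting behavior live in the game instance, so the component itself does no tracing or target detection.
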(event `self.ReceiveBeginPlay`
  (bind _asbp_game_instance (cast `/Game/Blueprint/BP_GameInstance` (`GameplayStatics.GetGameInstance`)))
  (set `self.BP Game Instance` _asbp_game_instance))

(event `EnhancedInput|/Game/ThirdPerson/Input/Actions/IA_Interact`
  (params (ActionValue :type Boolean) (ElapsedSeconds :type "Float (double-precision)") (TriggeredSeconds :type "Float (double-precision)") (InputAction :type "InputAction Object Reference" :default "/Game/ThirdPerson/Input/Actions/IA_Interact.IA_Interact"))
  (bind _bp_game_instance (`self.BP Game Instance`))
  (:`Started`
    (if (`/Game/Blueprint/BP_GameInstance.CanPress? ` _bp_game_instance)
      (`/Game/Blueprint/BP_GameInstance.ButtonPressed` _bp_game_instance)
      (elif (`/Game/Blueprint/BP_GameInstance.CanPressLight?` _bp_game_instance)
        (`/Game/Blueprint/BP_GameInstance.ButtonPressedLight` _bp_game_instance)))))