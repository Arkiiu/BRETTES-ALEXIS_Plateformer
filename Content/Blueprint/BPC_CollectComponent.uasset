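; BPC_CollectComponent is a component that handles picking up collectibles and scoring them.
; On BeginPlay it casts the game instance to BP_GameInstance and caches the reference.
; Collect adds the collectible's Value, scaled by the game instance's ScoreMultiplier, to the Score held there, then tells the collectible to destroy itself.
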(event `self.ReceiveBeginPlay`
  (bind _asbp_game_instance (cast `/Game/Blueprint/BP_GameInstance` (`GameplayStatics.GetGameInstance`)))
  (set `self.BP Game Instance` _asbp_game_instance))

(fn `Collect`
  (params (Collectible :type "/Game/Blueprint/BPC_CollectibleComponent Object Reference"))
  (bind _bp_game_instance (`self.BP Game Instance`))
  (set `/Game/Blueprint/BP_GameInstance.Score` (+ (* (`/Game/Blueprint/BPC_CollectibleComponent.Value` Collectible) (`/Game/Blueprint/BP_GameInstance.ScoreMultiplier` _bp_game_instance)) (`/Game/Blueprint/BP_GameInstance.Score` _bp_game_instance)) _bp_game_instance)
  (`/Game/Blueprint/BPC_CollectibleComponent.DestroyBPCollectible` Collectible))